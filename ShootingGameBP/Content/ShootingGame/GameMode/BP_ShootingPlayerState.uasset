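; BP_ShootingPlayerState is the player state for the shooting game, holding health, magazine count and user name.
; BeginPlay sets starting health and binds itself to the local player's BP_ShootingHud.
; Functions apply damage, add or spend magazines, check reload availability and set the name.
; RepNotify handlers on health, magazines and name fire event dispatchers with the new values, with the name change also printed on screen.
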(event EventBeginPlay
  (Variables|Default|SetCurHp 1e+02)
  (bind _asbp_shooting_hud (Utilities|Casting|CastToBP_ShootingHud (HUD|GetHUD (Game|GetPlayerController 0))))
  (Default|BindPlayerState _asbp_shooting_hud self))

(fn ConstructionScript)

(fn AddDamage
  (params (Damage :type Float%20%28double-precision%29))
  (Variables|Default|SetCurHp (- (Variables|Default|GetCurHp) Damage)))

(fn OnRepCurHp
  (Default|CallEventDispatcherUpdateHp (Variables|Default|GetCurHp) 1e+02))

(fn AddMag
  (Variables|Default|SetMag (+ (Variables|Default|GetMag) 1)))

(fn OnRepMag
  (Default|CallEventDispatcherUpdateMag (Variables|Default|GetMag)))

(fn UseMag
  (if (> (Variables|Default|GetMag) 0)
    (Variables|Default|SetMag (+ (Variables|Default|GetMag) -1))
    (return true)
    (else
      (return false))))

(fn IsCanReload
  (return (> (Variables|Default|GetMag) 0)))

(fn OnRepUserName
  (Development|PrintString (Utilities|String|Append "OnRep_UserName - " (Variables|Default|GetUserName)) true true "(R=0.000000,G=0.660000,B=1.000000,A=1.000000)" 6e+01)
  (Default|CallEventDispatcherUpdateUserName (Variables|Default|GetUserName)))

(fn SetUserName
  (params (UserName :type String))
  (Variables|Default|SetUserName UserName))