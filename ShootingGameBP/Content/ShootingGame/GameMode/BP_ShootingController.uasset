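; Player controller for the shooting game that hands the local user name to the player state on possession.
; Possess fires ResClinetPossess, which reads UserName from BP_ShootingGameInstance and passes it to ReqNewUserName.
; ReqNewUserName sets the name on BP_ShootingPlayerState; the Res/Req naming suggests a client-server round trip.
; Each step prints a long-lived debug message, while BeginPlay and Tick are empty.
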(event Custom|ResClinetPossess
  (Development|PrintString "ResClientPossess" true true "(R=0.000000,G=0.660000,B=1.000000,A=1.000000)" 6e+01)
  (bind _asbp_shooting_game_instance (Utilities|Casting|CastToBP_ShootingGameInstance (Game|GetGameInstance)))
  (CallFunction|ReqNewUserName (Variables|/Game/ShootingGame/GameMode/BP_ShootingGameInstance.BP_ShootingGameInstance_C|GetUserName _asbp_shooting_game_instance)))

(event Custom|ReqNewUserName
  (params (UserName :type String))
  (Development|PrintString (Utilities|String|Append "ReqNewUserName - " UserName) true true "(R=0.000000,G=0.660000,B=1.000000,A=1.000000)" 6e+01)
  (bind _asbp_shooting_player_state (Utilities|Casting|CastToBP_ShootingPlayerState (Variables|GetPlayerState)))
  (Default|SetUserName _asbp_shooting_player_state UserName))

(event EventBeginPlay)

(event EventTick
  (params (DeltaSeconds :type Float%20%28single-precision%29)))

(event EventPossess
  (params (PossessedPawn :type Pawn%20Object%20Reference))
  (Development|PrintString (Utilities|String|Append "On Possess - " (Utilities|GetDisplayName PossessedPawn)) true true "(R=0.000000,G=0.660000,B=1.000000,A=1.000000)" 6e+01)
  (CallFunction|ResClinetPossess))

(fn ConstructionScript)