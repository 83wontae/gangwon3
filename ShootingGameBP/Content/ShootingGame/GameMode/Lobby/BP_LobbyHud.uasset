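; Lobby HUD Blueprint that creates the lobby widget on BeginPlay and keeps its player list current.
; BindPlayerState hooks into a player state's user name dispatcher, prints a debug message and triggers an immediate update.
; Name updates ignore the passed name and call UpdatePlayerList on the widget.
; If the widget is not yet valid, a short timer retries the refresh by function name.
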(event EventBeginPlay
  (bind _returnvalue (UserInterface|CreateWidget "/Game/ShootingGame/Widget/Lobby/LobbyHudWidget.LobbyHudWidget_C"))
  (bind _output_get (Variables|Default|SetHudWidget _returnvalue))
  (UserInterface|Viewport|AddtoViewport _output_get 0))

(fn ConstructionScript)

(fn BindPlayerState
  (params (PlayerState :type BP%20Lobby%20Player%20State%20Object%20Reference))
  (EventDispatchers|BindEventtoEventDispatcherUserName PlayerState (EventDispatchers|CreateEvent :!event UpdateUserName))
  (Development|PrintString "BindPlayerState" true true "(R=0.000000,G=0.660000,B=1.000000,A=1.000000)" 6e+01)
  (CallFunction|UpdateUserName))

(fn UpdateUserName
  (params (UserName :type String))
  (CallFunction|UpdateUserNameHud))

(fn UpdateUserNameHud
  (bind _hudwidget (Variables|Default|GetHudWidget))
  (Utilities|IsValid _hudwidget
    (:Is%20Valid
      (Default|UpdatePlayerList _hudwidget))
    (:Is%20Not%20Valid
      (Utilities|Time|SetTimerbyFunctionName 0 "UpdateUserName_Hud" 0.01))))