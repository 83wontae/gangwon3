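; BP_MoveLeftRight is an actor that slides its StaticMesh back and forth along its relative X axis while IsPlay is true.
; Each Tick steps the X위치 (X position) variable by a fixed amount and writes it to the mesh's relative location.
; The 오른쪽방향진행 (moving right) flag sets the direction and flips at 0 and 200 units.
; The step ignores delta time, so speed depends on frame rate.
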(event EventBeginPlay)

(event EventTick
  (params (DeltaSeconds :type Float%20%28single-precision%29))
  (if (Variables|Default|GetIsPlay)
    (if (Variables|Default|Get오른쪽방향진행)
      ;[1 1 1] 오른쪽으로 이동
      (bind _output_get (Variables|Default|SetX위치 (+ (Variables|Default|GetX위치) 1.0)))
      (Transformation|SetRelativeLocation (Variables|Default|GetStaticMesh) (Math|Vector|MakeVector _output_get 0.0 0.0) false false)
      (if (>= (Variables|Default|GetX위치) 2e+02)
        (Variables|Default|Set오른쪽방향진행 false))
      (else
        ;[1 1 1] 왼쪽으로 이동
        (bind _output_get_2 (Variables|Default|SetX위치 (+ (Variables|Default|GetX위치) -1.0)))
        (Transformation|SetRelativeLocation (Variables|Default|GetStaticMesh) (Math|Vector|MakeVector _output_get_2 0.0 0.0) false false)
        (if (<= (Variables|Default|GetX위치) 0.0)
          (Variables|Default|Set오른쪽방향진행 true))))))

(fn ConstructionScript)